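; BP_Moon is a moon actor positioned at a radius around a target actor, or its spawn location if no target is valid.
; On BeginPlay it applies the first listed material and stores that location.
; Each Tick sets a Z-axis-rotated offset from StartAngle plus RotSpd, so the accumulated CurrRot never drives the orbit and the angle does not advance.
; An optional debug line links center and moon.
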(event EventBeginPlay
  (Utilities|FlowControl|Sequence
    (:then_0
      (CallFunction|ChangeMaterial))
    (:then_1
      (Variables|Handlers|SetInitialLoc (Transformation|GetActorLocation)))))

(event EventTick
  (params (DeltaSeconds :type Float%20%28single-precision%29))
  (Variables|Handlers|SetCurrRot (+ (Variables|Handlers|GetCurrRot) (* (* (Variables|Handlers|GetRotSpd) DeltaSeconds) (Math|Float|SelectFloat 1.0 -1.0 (Variables|Handlers|GetClockwise)))))
  (bind _newparam (CallFunction|RotateAroundObject self (Variables|Handlers|GetTarget) (Variables|Handlers|GetInitialLoc) (Variables|Handlers|GetRadius) (Variables|Handlers|GetStartAngle) (Variables|Handlers|GetRotSpd)))
  (if (Variables|Handlers|GetDrawDebug)
    (Rendering|Debug|DrawDebugLine _newparam (Transformation|GetActorLocation) (Variables|Handlers|GetTraceColor) 1.0 2.0)))

(fn ConstructionScript)

(fn ChangeMaterial
  (Rendering|Material|SetMaterial (Variables|Default|GetMoon) 0 (Utilities|Array|Get(acopy) (Variables|Materials|GetListOfMat))))

(fn RotateAroundObject
  (params (Actor%20to%20Rotate :type Actor%20Object%20Reference) (Target :type Actor%20Object%20Reference) (Target%20Location :type Vector) (Radius :type Float%20%28single-precision%29) (Angle :type Float%20%28single-precision%29) (Rotation%20Rate :type Float%20%28single-precision%29))
  (LocalVariables|SetLocal_ActorToRotate Actor%20to%20Rotate)
  (LocalVariables|SetLocal_Target Target)
  (LocalVariables|SetLocal_TargetLoc Target%20Location)
  (LocalVariables|SetLocal_Radius Radius)
  (LocalVariables|SetLocal_Angle Angle)
  (LocalVariables|SetLocal_RotationRate Rotation%20Rate)
  (Utilities|IsValid (LocalVariables|GetLocal_Target) ; If object exists, set target's location by grabbing our current location
    (:Is%20Valid
      (LocalVariables|SetLocal_TargetLoc (Transformation|GetActorLocation (LocalVariables|GetLocal_Target))))
    (:Is%20Not%20Valid
      _))
  (Transformation|SetActorLocation (LocalVariables|GetLocal_ActorToRotate) (+ (LocalVariables|GetLocal_TargetLoc) (Math|Vector|RotateVectorAroundAxis (Math|Vector|MakeVector (LocalVariables|GetLocal_Radius) 0.0 0.0) (+ (LocalVariables|GetLocal_Angle) (LocalVariables|GetLocal_RotationRate)) "0, 0,1.000000")) false false)
  (return (LocalVariables|GetLocal_TargetLoc)))