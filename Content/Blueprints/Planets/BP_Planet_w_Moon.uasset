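; Planet-with-moon actor Blueprint that varies the planet's appearance each time it begins play.
; On BeginPlay it sets a random material from the planet material list on the Planet component, then applies a material to the Moon component.
; The moon always gets the first entry of its material list, as its random index node is left unconnected.
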(event EventBeginPlay
  (Utilities|FlowControl|Sequence
    (:then_0
      (CallFunction|ChangeMaterialPlanet))
    (:then_1
      (CallFunction|ChangeMaterialMoon))))

(fn ConstructionScript)

(fn ChangeMaterialPlanet
  (bind _listofmat_planets (Variables|Materials|GetListOfMat_Planets))
  (Rendering|Material|SetMaterial (Variables|Default|GetPlanet) 0 (Utilities|Array|Get(acopy) _listofmat_planets (Math|Random|RandomInteger (+ (Utilities|Array|LastIndex _listofmat_planets) 1)))))

(fn ChangeMaterialMoon
  (Rendering|Material|SetMaterial (Variables|Default|GetMoon) 0 (Utilities|Array|Get(acopy) (Variables|Materials|GetListOfMat_Moons))))