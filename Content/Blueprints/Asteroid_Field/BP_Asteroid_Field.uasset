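; Actor that scatters a field of asteroids around its origin as instances of a single instanced static mesh component.
; The construction script loops up to a configurable count, placing each instance along a random direction at a random distance, producing a spherical shell.
; Each asteroid gets a random rotation and a random uniform scale adjusted by a multiplier, and the event graph holds no logic.
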(event EventBeginPlay)

(event Collision|EventActorBeginOverlap
  (params (OtherActor :type Actor%20Object%20Reference)))

(event EventTick
  (params (DeltaSeconds :type Float%20%28single-precision%29)))

(fn ConstructionScript
  (for _index (range 0 (Variables|Handlers|GetTotalAsteroids)) ; For each loop, create an instance mesh of asteroid
    (Components|InstancedStaticMesh|AddInstance (Variables|Default|GetInstancedStaticMesh) (Math|Transform|MakeTransform (* (Math|Random|RandomUnitVector) (Math|Random|RandomFloatinRange (Variables|Handlers|GetMinDis) (Variables|Handlers|GetMaxDis))) (Math|Random|RandomRotator false) (Math|Conversions|ToVector(Float) (* (Math|Random|RandomFloatinRange (Variables|Handlers|GetMinScale) (Variables|Handlers|GetMaxScale)) (Variables|Handlers|GetScaleMultiplier)))))))