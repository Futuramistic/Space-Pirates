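; Actor component that gives its owner health and destroys that actor when health reaches zero or below.
; On BeginPlay it binds to the owner's OnTakeAnyDamage and forwards the damage amount to a TakeDamage event, which subtracts it from Health without clamping.
; GetHealthPercentage returns Health divided by MaxHealth as a ratio.
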(event Custom|TakeDamage
  (params (DamageAmount :type Float%20%28single-precision%29))
  (bind _output_get (Variables|Default|SetHealth (- (Variables|Default|GetHealth) DamageAmount)))
  (if (<= _output_get 0.0)
    (Actor|DestroyActor (Variables|Default|GetOwner))))

(event Custom|CustomEvent_0
  (params (DamagedActor :type Actor%20Object%20Reference) (Damage :type Float%20%28single-precision%29) (DamageType :type Damage%20Type%20Object%20Reference) (InstigatedBy :type Controller%20Object%20Reference) (DamageCauser :type Actor%20Object%20Reference))
  (CallFunction|TakeDamage Damage))

(event EventBeginPlay
  (bind _output_get (Variables|Default|SetOwner (Components|GetOwner)))
  (EventDispatchers|BindEventtoOnTakeAnyDamage _output_get (delegate Custom|CustomEvent_0)))

(fn GetHealthPercentage
  (return (/ (Variables|Default|GetHealth) (Variables|Default|GetMaxHealth))))