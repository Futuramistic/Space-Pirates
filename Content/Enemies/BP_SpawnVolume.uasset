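; Volume actor that keeps spawning random enemies inside its box on a timer.
; A randomized initial cooldown staggers the first spawn, then Tick counts it down and resets it to the spawn interval after each spawn.
; SpawnRandom shuffles the enemy class array and spawns its first entry at a random point within the scaled box extent around the actor location.
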(event EventBeginPlay
  (Variables|Default|SetSpawnCooldown (Math|Random|RandomFloatinRange 0.0 (Variables|Default|GetSpawnInterval))))

(event Collision|EventActorBeginOverlap
  (params (OtherActor :type Actor%20Object%20Reference)))

(event EventTick
  (params (DeltaSeconds :type Float%20%28single-precision%29))
  (bind _output_get (Variables|Default|SetSpawnCooldown (- (Variables|Default|GetSpawnCooldown) DeltaSeconds)))
  (if (<= _output_get 0.0)
    (CallFunction|SpawnRandom)
    (Variables|Default|SetSpawnCooldown (Variables|Default|GetSpawnInterval))))

(fn ConstructionScript)

(fn SpawnRandom
  (bind _enemytypes (Variables|Default|GetEnemyTypes))
  (Utilities|Array|Shuffle _enemytypes)
  (Game|SpawnActorfromClass (Utilities|Array|Get(acopy) _enemytypes) (Math|Transform|MakeTransform (Math|Random|RandomPointinBoundingBox (Transformation|GetActorLocation) (Components|Box|GetScaledBoxExtent (Variables|Default|GetSpawnBox))) "0, 0, 0" "1,1,1") "Undefined" 0 0))