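; UFO enemy that chases the player pawn and shoots when within range.
; Tick interpolates rotation toward the player, moving closer beyond MinDistance or, within it, counting down a cooldown to fire forward from every mesh socket via BPCShootingEnemy.
; Hitting a SpaceShip damages both, zeroes its own loot drop, plays an explosion sound and offsets it along the hit normal.
; BeginPlay binds the health bar widget to BPCHealth.
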(event Custom|DamageSelf
  (params (Damage :type Float%20%28single-precision%29))
  ;[1 1 1] Damage on Collision with Spaceship
  (Default|SetDropAmount (Variables|Default|GetBPC_Lootable))
  (Game|Damage|ApplyDamage self Damage 0 0))

(event EventBeginPlay
  ;[1 1 1] Initialize Healthbar
  (bind _asui_health_bar (Utilities|Casting|CastToUI_HealthBar (UserInterface|GetUserWidgetObject (Variables|Default|GetHealthBar))))
  (Variables|/Game/Health/UI_HealthBar.UI_HealthBar_C|SetHealthObject _asui_health_bar (Variables|Default|GetBPC_Health)))

(event Collision|EventHit
  (params (MyComp :type Primitive%20Component%20Object%20Reference) (Other :type Actor%20Object%20Reference) (OtherComp :type Primitive%20Component%20Object%20Reference) (bSelfMoved :type Boolean) (HitLocation :type Vector :default "0, 0, 0") (HitNormal :type Vector :default "0, 0, 0") (NormalImpulse :type Vector :default "0, 0, 0") (Hit :type Hit%20Result%20Structure%20%28by%20ref%29))
  (bind _collisiondamage (Variables|Default|GetCollisionDamage))
  ;[1 1 1] Damage on Collision with Spaceship
  (bind _asspace_ship (Utilities|Casting|CastToSpaceShip Other))
  (Game|Damage|ApplyDamage _asspace_ship _collisiondamage 0 0)
  (CallFunction|DamageSelf _collisiondamage)
  (Audio|PlaySoundatLocation "/Game/StarterContent/Audio/Explosion_Cue.Explosion_Cue" (Transformation|GetActorLocation) "0, 0, 0" 1.0 1.0 0.0 0 0 0)
  (Transformation|AddActorWorldOffset (* HitNormal (* (Math|Vector|VectorLength (.BoxExtent (Collision|GetActorBounds false))) 1.5))))

(event EventTick
  (params (DeltaSeconds :type Float%20%28single-precision%29))
  (bind _returnvalue (Transformation|GetActorRotation))
  (bind _returnvalue_2 (Game|Player|GetPlayerPawn 0))
  (bind _returnvalue_3 (Transformation|GetActorLocation))
  (bind _rotatespeed (Variables|Default|GetRotateSpeed))
  (bind _returnvalue_4 (Transformation|GetActorLocation _returnvalue_2))
  (bind _returnvalue_5 (Math|Rotator|FindLookatRotation _returnvalue_3 _returnvalue_4))
  (bind _returnvalue_6 (Math|Interpolation|RInterpTo _returnvalue _returnvalue_5 DeltaSeconds _rotatespeed))
  ;[1 1 1] Simple AI that follows the player
  (if (Utilities|IsValid _returnvalue_2)
    (if (> (Math|Vector|Distance(Vector) _returnvalue_4 _returnvalue_3) (Variables|Default|GetMinDistance))
      (Pawn|Input|AddMovementInput (- _returnvalue_4 _returnvalue_3) 1.0 false)
      (Transformation|SetActorRotation _returnvalue_6)
      (else
        ;[1 1 1] Shoot when close enough
        (Transformation|SetActorRotation _returnvalue_6)
        (Variables|Default|SetFireRemainingCooldown (Math|Float|Max(Float) (- (Variables|Default|GetFireRemainingCooldown) (Utilities|Time|GetWorldDeltaSeconds)) 0.0))
        (CallFunction|Shoot)))))

(event Collision|EventActorBeginOverlap
  (params (OtherActor :type Actor%20Object%20Reference))
  ;[1 1 1] Damage on Collision with Spaceship
)

(fn ConstructionScript)

(fn Shoot
  (if (<= (Variables|Default|GetFireRemainingCooldown) 0.0)
    (Variables|Default|SetFireRemainingCooldown (Variables|Default|GetFireCooldown))
    (for _array_element (Transformation|GetAllSocketNames (Variables|Default|GetUFO%20mesh))
      (Default|EnemyShoot (Variables|Default|GetBPC_Shooting_Enemy) (Transformation|GetActorForwardVector) "0, 0, 0" (Transformation|GetSocketLocation (Variables|Default|GetUFO%20mesh) _array_element)))))