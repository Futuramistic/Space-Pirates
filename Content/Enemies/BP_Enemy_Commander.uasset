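; BP_Enemy_Commander is an enemy pawn that leads a group of soldiers, using a behavior tree and DoN navigation to move between goals.
; Damage from a non-enemy pawn makes it target the attacker, alert its soldiers, show its health bar and start firing.
; Tick spins the mesh and fires guided shots from every mesh socket on a cooldown.
; Colliding with a SpaceShip damages both and zeroes its loot drop.
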(event Custom|DamageSelf
  (params (Damage :type Float%20%28single-precision%29) (DamageCauser :type Pawn%20Object%20Reference))
  ;[1 1 1] Damage on Collision with Spaceship
  (Default|SetDropAmount (Variables|Default|GetBPC_Lootable))
  (Game|Damage|ApplyDamage self Damage 0 DamageCauser))

(event Custom|StartRunningBehaviourTree
  (bind _returnvalue (Class|DonNavigationHelper|DonNavigationManager))
  (bind _actorstoignoreforcollision (Variables|/Script/DonAINavigation.DonNavigationManager|GetActorsToIgnoreForCollision _returnvalue))
  ;[1 1 1] Start Running Behabior Tree
  (Utilities|FlowControl|Delay (Variables|Default|GetWake%20Up%20Delay))
  (Utilities|Array|Add _actorstoignoreforcollision (Variables|Default|GetGoal0))
  (Utilities|Array|Add _actorstoignoreforcollision (Variables|Default|GetGoal1))
  (if (not (Variables|Default|GetBT%20Initialized))
    (bind _asaicontroller (Utilities|Casting|CastToAIController (Pawn|GetController)))
    (AI|RunBehaviorTree _asaicontroller (Variables|Default|GetBehavior%20To%20Run))
    (Variables|Default|SetBT%20Initialized true)))

(event EventBeginPlay
  ;[1 1 1] Initialize Healthbar
  (bind _asui_health_bar (Utilities|Casting|CastToUI_HealthBar (UserInterface|GetUserWidgetObject (Variables|Default|GetHealthBar))))
  (Variables|/Game/Health/UI_HealthBar.UI_HealthBar_C|SetHealthObject _asui_health_bar (Variables|Default|GetBPC_Health))
  (Rendering|SetVisibility (Variables|Default|GetHealthBar) false false)
  (Variables|Default|SetFireRemainingCooldown (Math|Random|RandomFloatinRange 0.0 (Variables|Default|GetFireCoolDown))))

(event Collision|EventHit
  (params (MyComp :type Primitive%20Component%20Object%20Reference) (Other :type Actor%20Object%20Reference) (OtherComp :type Primitive%20Component%20Object%20Reference) (bSelfMoved :type Boolean) (HitLocation :type Vector :default "0, 0, 0") (HitNormal :type Vector :default "0, 0, 0") (NormalImpulse :type Vector :default "0, 0, 0") (Hit :type Hit%20Result%20Structure%20%28by%20ref%29))
  (bind _collision_damage (Variables|Default|GetCollision%20Damage))
  ;[1 1 1] Damage on Collision with Spaceship
  (bind _asspace_ship (Utilities|Casting|CastToSpaceShip Other))
  (Game|Damage|ApplyDamage _asspace_ship _collision_damage 0 self)
  (CallFunction|DamageSelf _collision_damage _asspace_ship)
  (Audio|PlaySoundatLocation "/Game/StarterContent/Audio/Explosion_Cue.Explosion_Cue" (Transformation|GetActorLocation) "0, 0, 0" 1.0 1.0 0.0 0 0 0)
  (Transformation|AddActorWorldOffset (* HitNormal (* (Math|Vector|VectorLength (.BoxExtent (Collision|GetActorBounds false))) 0.1))))

(event EventTick
  (params (DeltaSeconds :type Float%20%28single-precision%29))
  (bind _meshcomponent (Variables|GetMeshComponent))
  (bind _returnvalue (Transformation|GetWorldRotation _meshcomponent))
  (bind (_roll _pitch _yaw) (Math|Rotator|BreakRotator _returnvalue))
  (Transformation|SetWorldRotation _meshcomponent (Math|Interpolation|RInterpTo _returnvalue (Math|Rotator|MakeRotator (+ 45.0 _roll) _pitch _yaw) (Utilities|Time|GetWorldDeltaSeconds) 1.0) false false)
  ;[1 1 1] Shoot At Target
  (if (Variables|Default|GetIsFiring)
    (bind _pawn (CallFunction|GetGoalBot))
    (if (Utilities|IsValid _pawn)
      (Variables|Default|SetFireRemainingCooldown (Math|Float|Max(Float) (- (Variables|Default|GetFireRemainingCooldown) (Utilities|Time|GetWorldDeltaSeconds)) 0.0))
      (CallFunction|Shoot))))

(event EventAddMovementInputCustom
  (params (WorldDirection :type Vector :default "0, 0, 0") (ScaleValue :type Float%20%28single-precision%29))
  (bind _returnvalue (Math|Rotator|MakeRotfromX WorldDirection))
  (bind (_roll _pitch _yaw) (Math|Rotator|BreakRotator _returnvalue))
  ;[1 1 1] Movement
  (Transformation|SetActorRotation (Math|Interpolation|RInterpTo (Transformation|GetActorRotation) (Math|Rotator|MakeRotator (Math|Float|Clamp(Float) _roll -3e+01 3e+01) (Math|Float|Clamp(Float) _pitch -3e+01 3e+01) _yaw) (Utilities|Time|GetWorldDeltaSeconds) 5.0))
  (Pawn|Input|AddMovementInput WorldDirection (* ScaleValue (Variables|Default|GetBot%20Speed%20Scale)) false))

(event EventNotifyTarget
  (params (Target :type Pawn%20Object%20Reference))
  ;[1 1 1] Notify all soldiers and self
  (if (not (Variables|Default|GetIsNotified))
    (for _array_element (Variables|Default|GetSoldierArray)
      (Utilities|IsValid _array_element
        (:Is%20Valid
          (Default|NotifyTarget _array_element Target))))
    (Utilities|Array|Add (Variables|/Script/DonAINavigation.DonNavigationManager|GetActorsToIgnoreForCollision (Class|DonNavigationHelper|DonNavigationManager)) Target)
    (Variables|Default|SetGoal%20Bot Target)
    (Variables|Default|SetIsFiring true)
    (Variables|Default|SetIsNotified true)
    (Rendering|SetVisibility (Variables|Default|GetHealthBar) true false)))

(event Game|Damage|EventAnyDamage
  (params (Damage :type Float%20%28single-precision%29) (DamageType :type Damage%20Type%20Object%20Reference) (InstigatedBy :type Controller%20Object%20Reference) (DamageCauser :type Actor%20Object%20Reference))
  ;[1 1 1] Chase player and notify soldiers when damaged
  (bind _aspawn (Utilities|Casting|CastToPawn DamageCauser))
  (if (!= _aspawn self)
    (if (not (Actor|ActorHasTag _aspawn "Enemy"))
      (CallFunction|NotifyTarget _aspawn))))

(event EventCallTriggerActor)

(event EventCallTriggerActorEndOverlap)

(fn ConstructionScript)

(fn Shoot
  (if (<= (Variables|Default|GetFireRemainingCooldown) 0.0)
    (Variables|Default|SetFireRemainingCooldown (Variables|Default|GetFireCooldown))
    (for _array_element (Transformation|GetAllSocketNames (Variables|GetMeshComponent))
      (bind _pawn (CallFunction|GetGoalBot))
      (Utilities|IsValid _pawn
        (:Is%20Valid
          (Default|EnemyShoot (Variables|Default|GetBPC_Shooting_Guided_Enemy) (Transformation|GetActorForwardVector) "0, 0, 0" (Transformation|GetSocketLocation (Variables|GetMeshComponent) _array_element) _pawn))
        (:Is%20Not%20Valid
          (Development|PrintString "Hello"))))))

(fn GetGoalActor
  (bind _goals (Variables|Default|GetGoals))
  (bind _returnvalue (Utilities|Array|Length _goals))
  (if (>= (+ (Variables|Default|GetLastGoalIndex) (Math|Random|RandomIntegerinRange 1 1)) _returnvalue)
    (bind _output_get (Variables|Default|SetLastGoalIndex (- (+ (Variables|Default|GetLastGoalIndex) (Math|Random|RandomIntegerinRange 1 1)) _returnvalue)))
    (return (Utilities|Array|Get(acopy) (Variables|Default|GetGoals) _output_get))
    (else
      (bind _output_get_2 (Variables|Default|SetLastGoalIndex (+ (Variables|Default|GetLastGoalIndex) (Math|Random|RandomIntegerinRange 1 1))))
      (return (Utilities|Array|Get(acopy) (Variables|Default|GetGoals) _output_get_2)))))

(fn GetGoalBot
  (return (Variables|Default|GetGoal%20Bot)))

(fn Notified
  (return (Variables|Default|GetIsNotified)))

(fn OnGoalReached
  (return (Variables|Default|GetGoal%20Cooldown%20Time) true))