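; BP_Enemy is an enemy actor that deals collision damage to the player's SpaceShip.
; On BeginPlay it binds its health component to the UI_HealthBar widget shown by its HealthBar component.
; Overlapping a SpaceShip applies CollisionDamage to both the ship and itself through DamageSelf, then plays an explosion sound at its location.
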(event OnComponentHit(Box)
  (params (HitComponent :type Primitive%20Component%20Object%20Reference) (OtherActor :type Actor%20Object%20Reference) (OtherComp :type Primitive%20Component%20Object%20Reference) (NormalImpulse :type Vector :default "0, 0, 0") (Hit :type Hit%20Result%20Structure%20%28by%20ref%29)))

(event Custom|DamageSelf
  (params (Damage :type Float%20%28single-precision%29))
  (Game|Damage|ApplyDamage self Damage 0 0))

(event EventBeginPlay
  (bind _asui_health_bar (Utilities|Casting|CastToUI_HealthBar (UserInterface|GetUserWidgetObject (Variables|Default|GetHealthBar))))
  (Variables|/Game/Health/UI_HealthBar.UI_HealthBar_C|SetHealthObject _asui_health_bar (Variables|Default|GetBPC_Health)))

(event EventTick
  (params (DeltaSeconds :type Float%20%28single-precision%29)))

(event Collision|EventActorBeginOverlap
  (params (OtherActor :type Actor%20Object%20Reference))
  (bind _collisiondamage (Variables|Default|GetCollisionDamage))
  (bind _asspace_ship (Utilities|Casting|CastToSpaceShip OtherActor))
  (Game|Damage|ApplyDamage _asspace_ship _collisiondamage 0 0)
  (CallFunction|DamageSelf _collisiondamage)
  (Audio|PlaySoundatLocation "/Game/StarterContent/Audio/Explosion02.Explosion02" (Transformation|GetActorLocation) "0, 0, 0" 1.0 1.0 0.0 0 0 0))

(fn ConstructionScript)