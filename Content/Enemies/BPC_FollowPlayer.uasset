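; Actor component that gives an enemy Pawn simple AI to follow the player.
; BeginPlay caches the owning actor as a Pawn.
; Each Tick, if player pawn 0 is valid, it feeds movement input toward that pawn using the unnormalized offset, scaled by MoveSpeed.
; When RotationSpeed is non-zero, it also turns the owner toward the player at a constant rate with RInterpToConstant.
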(event EventBeginPlay
  (bind _aspawn (Utilities|Casting|CastToPawn (Components|GetOwner)))
  (Variables|Default|SetOwner _aspawn))

(event EventTick
  (params (DeltaSeconds :type Float%20%28single-precision%29))
  (bind _returnvalue (Game|Player|GetPlayerPawn 0))
  (bind _rotationspeed (Variables|Default|GetRotationSpeed))
  (bind _owner (Variables|Default|GetOwner))
  (bind _owner_2 (Variables|Default|GetOwner))
  (bind _returnvalue_2 (Transformation|GetActorLocation _returnvalue))
  (bind _returnvalue_3 (Transformation|GetActorLocation _owner))
  ;[1 1 1] Simple AI that follows the player
  (if (Utilities|IsValid _returnvalue)
    (Pawn|Input|AddMovementInput _owner_2 (- _returnvalue_2 _returnvalue_3) (Variables|Default|GetMoveSpeed) false)
    (if (not (== _rotationspeed 0.0))
      (Transformation|SetActorRotation _owner_2 (Class|KismetMathLibrary|RInterptoConstant (Transformation|GetActorRotation _owner) (Math|Rotator|FindLookatRotation _returnvalue_3 _returnvalue_2) DeltaSeconds _rotationspeed)))))