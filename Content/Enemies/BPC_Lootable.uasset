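; BPC_Lootable is an actor component that makes its owner drop loot when destroyed.
; On BeginPlay it binds to the owner's OnDestroyed event, which calls SpawnLootItem at the owner's location.
; SpawnLootItem spawns DropAmount copies of the LootItem class, each offset 50 units in a random direction.
; SetDropAmount lets other code change the drop count.
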(event Custom|CustomEvent_0
  (params (DestroyedActor :type Actor%20Object%20Reference))
  (CallFunction|SpawnLootItem (Transformation|GetActorLocation (Variables|Default|GetOwner))))

(event EventBeginPlay
  (bind _output_get (Variables|Default|SetOwner (Components|GetOwner)))
  (Game|BindEventtoOnDestroyed _output_get (delegate Custom|CustomEvent_0)))

(event EventTick
  (params (DeltaSeconds :type Float%20%28single-precision%29)))

(fn SpawnLootItem
  (params (SpawnLocation :type Vector))
  (for _index (range 1 (Variables|Default|GetDropAmount))
    (Game|SpawnActorfromClass (Variables|Default|GetLootItem) (Math|Transform|MakeTransform (+ SpawnLocation (* (Math|Random|RandomUnitVector) 5e+01)) "0, 0, 0" "1,1,1") "Undefined" 0 0)))

(fn SetDropAmount
  (params (DropAmount :type Integer))
  (Variables|Default|SetDropAmount DropAmount))