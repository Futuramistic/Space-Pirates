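; Boss cruiser enemy with a floating health bar and point-defense guns that shoot at the player.
; On BeginPlay it binds the health bar widget to its health component.
; Tick polls two cooldown components; point defense fires from each child mount within range of the player via the shooting component, while the main cannon branch does nothing yet.
; The shared Fire function treats zero range as unlimited.
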(event EventBeginPlay
  ;[1 1 1] Initialize Healthbar
  (bind _asui_health_bar (Utilities|Casting|CastToUI_HealthBar (UserInterface|GetUserWidgetObject (Variables|Default|GetHealthBar))))
  (Variables|/Game/Health/UI_HealthBar.UI_HealthBar_C|SetHealthObject _asui_health_bar (Variables|Default|GetBPC_Health))
  (Default|SetSize _asui_health_bar 1e+01))

(event Collision|EventActorBeginOverlap
  (params (OtherActor :type Actor%20Object%20Reference))
  (|CallParentFunction OtherActor) ; This node is disabled and will not be called.\nDrag off pins to build functionality.
)

(event EventTick
  (params (DeltaSeconds :type Float%20%28single-precision%29))
  (Utilities|FlowControl|Sequence
    (:then_0
      (if (Default|Fire (Variables|Default|GetBPC_Cooldown_MainCannon))
        _))
    (:then_1
      (if (Default|Fire (Variables|Default|GetBPC_Cooldown_PointDefense))
        (CallFunction|Fire (Components|GetChildrenComponents (Variables|Default|GetPointDefense) false) 1.2e+04)))))

(fn ConstructionScript
  (|CallParentFunction))

(fn Fire
  (params (Components :type Array%20of%20Scene%20Component%20Object%20References) (Range :type Float%20%28single-precision%29))
  (for _array_element Components
    (if (or (<= (Math|Vector|Distance(Vector) (- (Transformation|GetActorLocation (Game|Player|GetPlayerPawn 0)) (Transformation|GetWorldLocation _array_element)) "0, 0, 0") Range) (== Range 0.0))
      (Default|EnemyShoot (Variables|Default|GetBPC_Shooting_Enemy) (- (Transformation|GetActorLocation (Game|Player|GetPlayerPawn 0)) (Transformation|GetWorldLocation _array_element)) "0, 0, 0" (Transformation|GetWorldLocation _array_element)))))