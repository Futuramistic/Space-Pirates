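; Enemy group spawner that periodically creates a commander and a squad of soldiers at random points inside its SpawnBox, after a randomized first delay.
; BeginPlay places hidden goal cues around the box, which are handed to every spawned enemy.
; SpawnRandom chains soldiers into a follow hierarchy through GoalBot, rooted at the commander, then starts their behavior trees.
; SpawnRocks can scatter nav obstacles but is never called here.
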(event EventBeginPlay
  (Variables|Default|SetSpawnCooldown (Math|Random|RandomFloatinRange 0.0 (Variables|Default|GetSpawnInterval)))
  (CallFunction|InitGoalTransforms)
  (for _array_element (Variables|Default|GetGoalTransforms)
    (bind _returnvalue (Game|SpawnActorfromClass "/Game/Enemies/DonNavigationSamples/Blueprints/Cues/GoalCue.GoalCue_C" _array_element "AlwaysSpawn" 0 0))
    (Utilities|Array|Add (Variables|Default|GetGoals) _returnvalue)
    (Rendering|SetVisibility (Variables|/Game/Enemies/DonNavigationSamples/Blueprints/Cues/GoalCue.GoalCue_C|GetScene _returnvalue) false true)))

(event Collision|EventActorBeginOverlap
  (params (OtherActor :type Actor%20Object%20Reference)))

(event EventTick
  (params (DeltaSeconds :type Float%20%28single-precision%29))
  (bind _output_get (Variables|Default|SetSpawnCooldown (- (Variables|Default|GetSpawnCooldown) DeltaSeconds)))
  (if (<= _output_get 0.0)
    (CallFunction|SpawnRandom)
    (Variables|Default|SetSpawnCooldown (Variables|Default|GetSpawnInterval))))

(fn ConstructionScript)

(fn SpawnRandom
  (bind _returnvalue (Transformation|GetActorLocation))
  (bind _spawnbox (Variables|Default|GetSpawnBox))
  (bind _soldiers (Variables|Default|GetSoldiers))
  (bind _returnvalue_2 (Components|Box|GetScaledBoxExtent _spawnbox))
  (bind _output (Utilities|Array|Get(acopy) _soldiers))
  (bind _returnvalue_3 (Math|Random|RandomPointinBoundingBox _returnvalue _returnvalue_2))
  (Utilities|Array|Clear (Variables|Default|GetSoldiers))
  (for (_array_element _array_index) (Variables|Default|GetEnemyTypes)
    (for _index (range 0 (* _array_index 5))
      (switch int _array_index
        (:0
          (bind _returnvalue_4 (AI|SpawnAIFromClass _array_element "/Game/Enemies/DonNavigationSamples/Blueprints/BehaviorTree/BT_GoThroughGoals.BT_GoThroughGoals" _returnvalue_3 "0, 0, 0" false))
          (bind _asbp_enemy_commander (Utilities|Casting|CastToBP_Enemy_Commander _returnvalue_4))
          (Variables|Default|SetCommander _asbp_enemy_commander))
        (:1
          (bind _returnvalue_5 (AI|SpawnAIFromClass _array_element "/Game/Enemies/DonNavigationSamples/Blueprints/BehaviorTree/BT_Chase_Randomized.BT_Chase_Randomized" _returnvalue_3 "0, 0, 0" false))
          (bind _asbp_enemy_soldier (Utilities|Casting|CastToBP_Enemy_Soldier _returnvalue_5))
          (Utilities|Array|Add (Variables|Default|GetSoldiers) _asbp_enemy_soldier)))))
  ;[1 1 1] Init soldier and start running behaviour tree
  (for (_array_element_2 _array_index_2) (Variables|Default|GetSoldiers)
    (switch int _array_index_2
      (:Default
        (Variables|/Game/Enemies/BP_Enemy_Soldier.BP_Enemy_Soldier_C|SetGoal%20Bot _array_element_2 (Variables|Default|GetCommander)))
      (:0
        (Variables|/Game/Enemies/BP_Enemy_Soldier.BP_Enemy_Soldier_C|SetGoal%20Bot _array_element_2 (Variables|Default|GetCommander)))
      (:1
        (Variables|/Game/Enemies/BP_Enemy_Soldier.BP_Enemy_Soldier_C|SetGoal%20Bot _array_element_2 _output))
      (:2
        (Variables|/Game/Enemies/BP_Enemy_Soldier.BP_Enemy_Soldier_C|SetGoal%20Bot _array_element_2 _output))
      (:3
        (Variables|/Game/Enemies/BP_Enemy_Soldier.BP_Enemy_Soldier_C|SetGoal%20Bot _array_element_2 (Utilities|Array|Get(acopy) _soldiers 1)))
      (:4
        (Variables|/Game/Enemies/BP_Enemy_Soldier.BP_Enemy_Soldier_C|SetGoal%20Bot _array_element_2 (Utilities|Array|Get(acopy) _soldiers 2)))
      (:5
        (Variables|/Game/Enemies/BP_Enemy_Soldier.BP_Enemy_Soldier_C|SetGoal%20Bot _array_element_2 (Utilities|Array|Get(acopy) _soldiers 3))))
    (Variables|/Game/Enemies/BP_Enemy_Soldier.BP_Enemy_Soldier_C|SetCommander _array_element_2 (Variables|Default|GetCommander))
    (Variables|/Game/Enemies/BP_Enemy_Soldier.BP_Enemy_Soldier_C|SetGoals _array_element_2 (Variables|Default|GetGoals))
    (Variables|/Game/Enemies/BP_Enemy_Soldier.BP_Enemy_Soldier_C|SetBehavior%20To%20Run _array_element_2 "/Game/Enemies/DonNavigationSamples/Blueprints/BehaviorTree/BT_Chase_Randomized.BT_Chase_Randomized")
    (Default|StartRunningBehaviourTree _array_element_2))
  ;[1 1 1] Init commander and start running behaviour tree
  (Variables|/Game/Enemies/BP_Enemy_Commander.BP_Enemy_Commander_C|SetGoals (Variables|Default|GetCommander) (Variables|Default|GetGoals))
  (Variables|/Game/Enemies/BP_Enemy_Commander.BP_Enemy_Commander_C|SetSoldierArray (Variables|Default|GetCommander) (Variables|Default|GetSoldiers))
  (Default|StartRunningBehaviourTree (Variables|Default|GetCommander)))

(fn InitGoalTransforms
  (bind _spawnbox (Variables|Default|GetSpawnBox))
  (bind _goaltransforms (Variables|Default|GetGoalTransforms))
  (bind _spawnbox_2 (Variables|Default|GetSpawnBox))
  (bind _returnvalue (Components|Box|GetScaledBoxExtent _spawnbox))
  (bind _returnvalue_2 (Components|Box|GetScaledBoxExtent _spawnbox_2))
  (Utilities|Array|Add _goaltransforms (Math|Conversions|ToTransform(Vector) (+ (Transformation|GetActorLocation) (Components|Box|GetScaledBoxExtent (Variables|Default|GetSpawnBox)))))
  (Utilities|Array|Add _goaltransforms (Math|Conversions|ToTransform(Vector) (- (Transformation|GetActorLocation) (Components|Box|GetScaledBoxExtent (Variables|Default|GetSpawnBox)))))
  (Utilities|Array|Add _goaltransforms (Math|Conversions|ToTransform(Vector) (+ (Transformation|GetActorLocation) (Math|Vector|MakeVector (.x _returnvalue_2) 0.0 (* (.z _returnvalue_2) -1.0)))))
  (Utilities|Array|Add _goaltransforms (Math|Conversions|ToTransform(Vector) (+ (Transformation|GetActorLocation) (Math|Vector|MakeVector (* (.x _returnvalue) -1.0) 0.0 (.z _returnvalue))))))

(fn SpawnRocks
  (for _index (range 0 10)
    (Game|SpawnActorfromClass "/Game/Enemies/DonNavigationSamples/Blueprints/DynamicObstacles/BP_NAV_Obstacle.BP_NAV_Obstacle_C" (Math|Conversions|ToTransform(Vector) (Math|Random|RandomPointinBoundingBox (Transformation|GetActorLocation) (Components|Box|GetScaledBoxExtent (Variables|Default|GetSpawnBox)))) "Undefined" 0 0)))