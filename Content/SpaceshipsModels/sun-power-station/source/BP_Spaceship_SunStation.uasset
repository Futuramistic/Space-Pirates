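; BP_Spaceship_SunStation is a sun power station model that animates itself with continuously spinning parts.
; Tick adds small fixed relative rotations to geosphere and shape components, mostly in matched pairs, each on its own axis and speed.
; The increments are not scaled by delta time, so spin speed follows frame rate.
; BeginPlay fills a RotatingElements array with the geospheres, but Tick rotates components directly instead of reading it.
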(event EventBeginPlay
  (bind _rotating_elements (Variables|Default|Getrotating_elements))
  (Utilities|Array|Add _rotating_elements (Variables|Default|GetSun_Power_Station_GeoSphere004))
  (Utilities|Array|Add _rotating_elements (Variables|Default|GetSun_Power_Station_GeoSphere003))
  (Utilities|Array|Add _rotating_elements (Variables|Default|GetSun_Power_Station_GeoSphere002))
  (Utilities|Array|Add _rotating_elements (Variables|Default|GetSun_Power_Station_GeoSphere005)))

(event Collision|EventActorBeginOverlap
  (params (OtherActor :type Actor%20Object%20Reference)))

(event EventTick
  (params (DeltaSeconds :type Float%20%28single-precision%29))
  (Transformation|AddRelativeRotation (Variables|Default|GetSun_Power_Station_GeoSphere005) (Math|Rotator|MakeRotator 0.01 0.0 0.0) false false)
  (Transformation|AddRelativeRotation (Variables|Default|GetSun_Power_Station_Shape002) (Math|Rotator|MakeRotator 0.01 0.0 0.0) false false)
  (Transformation|AddRelativeRotation (Variables|Default|GetSun_Power_Station_GeoSphere003) (Math|Rotator|MakeRotator 0.0 0.02 0.0) false false)
  (Transformation|AddRelativeRotation (Variables|Default|GetSun_Power_Station_Shape) (Math|Rotator|MakeRotator 0.0 0.02 0.0) false false)
  (Transformation|AddRelativeRotation (Variables|Default|GetSun_Power_Station_GeoSphere004) (Math|Rotator|MakeRotator 0.0 0.0 0.03) false false)
  (Transformation|AddRelativeRotation (Variables|Default|GetSun_Power_Station_Shape001) (Math|Rotator|MakeRotator 0.0 0.0 0.03) false false)
  (Transformation|AddRelativeRotation (Variables|Default|GetSun_Power_Station_GeoSphere002) (Math|Rotator|MakeRotator 0.05 0.0 0.0) false false))

(fn ConstructionScript)