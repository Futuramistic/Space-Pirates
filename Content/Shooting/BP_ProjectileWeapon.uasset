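; BP_ProjectileWeapon is a weapon Blueprint that fires projectiles from its Arrow component, rate-limited by a cooldown component.
; The construction script passes Cooldown to BPCCooldown, whose Fire check gates each Fire event.
; Each shot spawns at least one ProjectileClass actor per MultishotCount, randomizing direction within a Spread-degree cone and passing on Instigator and Damage.
; One shot sound then plays at the arrow, however many projectiles spawn.
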(event EventBeginPlay)

(event Collision|EventActorBeginOverlap
  (params (OtherActor :type Actor%20Object%20Reference)))

(event EventTick
  (params (DeltaSeconds :type Float%20%28single-precision%29)))

(event EventFire
  (params (Instigator :type Pawn%20Object%20Reference))
  (if (Default|Fire (Variables|Default|GetBPC_Cooldown))
    (CallFunction|Fire Instigator)))

(fn ConstructionScript
  (Default|SetCooldown (Variables|Default|GetBPC_Cooldown) (Variables|Default|GetCooldown)))

(fn CanFire
  (return true))

(fn Fire
  (params (Instigator :type Pawn%20Object%20Reference))
  (bind _arrow (Variables|Default|GetArrow))
  (bind _returnvalue (Transformation|GetWorldTransform _arrow))
  ;[1 1 1] Fire #multishot projectiles with spread, then play shot sound
  (for _index (range 1 (Math|Integer|Max(Integer) (Math|Float|Truncate (Variables|Default|GetMultishotCount)) 1))
    (bind _modifiedrotation (CallFunction|CalculateRandomSpread (.rotation _returnvalue)))
    (bind _returnvalue_2 (Game|SpawnActorfromClass (Variables|Default|GetProjectileClass) (Math|Transform|MakeTransform (.location _returnvalue) _modifiedrotation (.scale _returnvalue)) "AlwaysSpawn" 0 Instigator))
    (Default|SetDamage _returnvalue_2 (Variables|Default|GetDamage)))
  (Audio|PlaySoundatLocation "/Game/Audio/ShotSound.ShotSound" (.location _returnvalue) "0, 0, 0" 1.0 1.0 0.0 0 0 0))

(fn CalculateRandomSpread
  (params (BaseRotation :type Rotator))
  (return (Math|Conversions|RotationFromXVector (Math|Random|RandomUnitVectorinConeinDegrees (Math|Vector|GetForwardVector BaseRotation) (Variables|Default|GetSpread)))))