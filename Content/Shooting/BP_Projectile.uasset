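; BP_Projectile is a shot actor that damages whatever it hits and then destroys itself.
; On BeginPlay its Sphere ignores the instigator while moving and a timer starts for its Lifetime.
; When the timer runs out, Expire disables the BPCExplodesOnDeath component before destroying the actor, while a hit leaves that component untouched.
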(event EventBeginPlay
  (Collision|IgnoreActorwhenMoving (Variables|Default|GetSphere) (Game|GetInstigator) true)
  (Utilities|Time|SetTimerbyFunctionName 0 "Expire" (Variables|Default|GetLifetime)))

(event EventTick
  (params (DeltaSeconds :type Float%20%28single-precision%29)))

(event Collision|EventHit
  (params (MyComp :type Primitive%20Component%20Object%20Reference) (Other :type Actor%20Object%20Reference) (OtherComp :type Primitive%20Component%20Object%20Reference) (bSelfMoved :type Boolean) (HitLocation :type Vector :default "0, 0, 0") (HitNormal :type Vector :default "0, 0, 0") (NormalImpulse :type Vector :default "0, 0, 0") (Hit :type Hit%20Result%20Structure%20%28by%20ref%29))
  (Game|Damage|ApplyDamage Other (Variables|Default|GetDamage) 0 0)
  (Actor|DestroyActor))

(fn ConstructionScript)

(fn Expire
  (Default|Disable (Variables|Default|GetBPC_ExplodesOnDeath))
  (Actor|DestroyActor))