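; Beam weapon actor that applies damage scaled by frame time to whatever it hits along the arrow's forward direction within Range.
; FindTarget line-traces on the Beam profile and, unless that hits a Pawn, falls back to a sphere trace for soft-lock aiming.
; UpdateBeam stretches and rotates a mesh to the impact point or maximum range, using bounds cached at construction.
; EndFire hides the beam by passing a zero-length target.
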(event EventBeginPlay
  (|CallParentFunction) ; This node is disabled and will not be called.\nDrag off pins to build functionality.
)

(event Collision|EventActorBeginOverlap
  (params (OtherActor :type Actor%20Object%20Reference))
  (|CallParentFunction OtherActor) ; This node is disabled and will not be called.\nDrag off pins to build functionality.
)

(event EventTick
  (params (DeltaSeconds :type Float%20%28single-precision%29))
  (|CallParentFunction DeltaSeconds))

(event EventEndFire
  (params (Instigator :type Pawn%20Object%20Reference))
  (CallFunction|UpdateBeam (Transformation|GetWorldLocation (Variables|Default|GetArrow))))

(event EventFire
  (params (Instigator :type Pawn%20Object%20Reference))
  (bind _canfire (CallFunction|CanFire))
  (if _canfire
    (CallFunction|Fire Instigator)))

(fn ConstructionScript
  (bind _sm_beam (Variables|Default|GetSM_Beam))
  (bind (_min _max) (Components|StaticMesh|GetLocalBounds _sm_beam))
  (|CallParentFunction)
  (Variables|Default|SetInitialScale (Transformation|GetWorldScale (Variables|Default|GetSM_Beam)))
  (Variables|Default|SetSizeX (Math|Float|Absolute(Float) (.x (- _min _max)))))

(fn CanFire
  (return true))

(fn Fire
  (params (Instigator :type Pawn%20Object%20Reference))
  (bind _arrow (Variables|Default|GetArrow))
  (bind _range (Variables|Default|GetRange))
  (bind _returnvalue (Transformation|GetWorldLocation _arrow))
  (bind _returnvalue_2 (Math|Vector|GetForwardVector _arrow))
  (bind _returnvalue_3 (* _returnvalue_2 _range))
  (bind _returnvalue_4 (+ _returnvalue _returnvalue_3))
  (bind (_outhit_impactpoint _outhit_hitactor _returnvalue_5) (CallFunction|FindTarget _returnvalue _returnvalue_4 (Variables|Default|GetSoftlockSize) (Utilities|Array|MakeArray Instigator)))
  (if _returnvalue_5
    (CallFunction|UpdateBeam _outhit_impactpoint)
    (Game|Damage|ApplyDamage _outhit_hitactor (* (Variables|Default|GetDamagePerSecond) (Utilities|Time|GetWorldDeltaSeconds)) 0 Instigator)
    (else
      (CallFunction|UpdateBeam _returnvalue_4))))

(fn UpdateBeam
  (params (Target :type Vector))
  (bind _sm_beam (Variables|Default|GetSM_Beam))
  (bind _initialscale (Variables|Default|GetInitialScale))
  (bind _arrow (Variables|Default|GetArrow))
  (bind _returnvalue (Transformation|GetWorldLocation _arrow))
  (bind _returnvalue_2 (- Target _returnvalue))
  (bind _returnvalue_3 (Math|Vector|VectorLength _returnvalue_2))
  (if (<= _returnvalue_3 0.0)
    (Rendering|SetVisibility _sm_beam false false)
    (else
      (Transformation|SetWorldScale3D (Variables|Default|GetSM_Beam) (Math|Vector|MakeVector (/ _returnvalue_3 (Variables|Default|GetSizeX)) (.y _initialscale) (.z _initialscale)))
      (Rendering|SetVisibility _sm_beam true false)
      (Transformation|SetWorldRotation (Variables|Default|GetSM_Beam) (Math|Conversions|RotationFromXVector _returnvalue_2) false false))))

(fn FindTarget
  (params (Start :type Vector) (End :type Vector) (Radius :type Float%20%28single-precision%29) (ActorsToIgnore :type Array%20of%20Actor%20Object%20References))
  ;[1 1 1] First try line trace, then try sphere trace
  (bind (_outhit _returnvalue) (Class|KismetSystemLibrary|LineTraceSinglebyProfile Start End "Beam" false ActorsToIgnore "None" true))
  (Utilities|Casting|CastToPawn (.hitactor _outhit)
    (:then
      (return (.impactpoint _outhit) (.hitactor _outhit) _returnvalue))
    (:CastFailed
      (bind (_outhit_2 _returnvalue_2) (Class|KismetSystemLibrary|SphereTraceSinglebyProfile Start End Radius "Beam" false ActorsToIgnore "None" true))
      (return (.impactpoint _outhit_2) (.hitactor _outhit_2) _returnvalue_2))))