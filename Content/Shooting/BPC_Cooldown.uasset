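; Cooldown component for shooting that gates how often an action can fire.
; Tick counts CooldownRemaining down to zero, scaled by an adjustable CooldownRate.
; Fire succeeds only when IsReady reports zero remaining, then resets the timer to Cooldown and returns whether it fired.
; Getters and setters expose the cooldown length and rate, plus read-only access to the remaining time.
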(event EventBeginPlay)

(event EventTick
  (params (DeltaSeconds :type Float%20%28single-precision%29))
  (Variables|Default|SetCooldownRemaining (Math|Float|Max(Float) (- (Variables|Default|GetCooldownRemaining) (* DeltaSeconds (Variables|Default|GetCooldownRate))) 0.0)))

(fn GetCooldown
  (return (Variables|Default|GetCooldown)))

(fn SetCooldown
  (params (Cooldown :type Float%20%28single-precision%29))
  (Variables|Default|SetCooldown Cooldown)
  (return))

(fn GetCooldownRemaining
  (return (Variables|Default|GetCooldownRemaining)))

(fn Fire
  (if (CallFunction|IsReady)
    (Variables|Default|SetCooldownRemaining (Variables|Default|GetCooldown))
    (return true)
    (else
      (return false))))

(fn GetCooldownRate
  (return (Variables|Default|GetCooldownRate)))

(fn SetCooldownRate
  (params (CooldownRate :type Float%20%28single-precision%29))
  (Variables|Default|SetCooldownRate CooldownRate)
  (return))

(fn IsReady
  (return (<= (CallFunction|GetCooldownRemaining) 0.0)))